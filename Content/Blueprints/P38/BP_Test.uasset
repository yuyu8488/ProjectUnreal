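; BP_Test is a test actor Blueprint with a function that rotates the actor from roll, pitch and yaw inputs.
; UpdateRotation lerps the current rotation, as a vector, toward the inputs scaled by RotationSpeed, using a delta-time-based alpha.
; It applies that blend as an added world rotation delta rather than an absolute rotation.
; An equivalent SetActorRotation node sits disconnected, and nothing shown calls UpdateRotation.
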(fn `UpdateRotation`
  (bind (_returnvalue_roll _returnvalue_pitch _returnvalue_yaw) (`KismetMathLibrary.BreakRotator` (`self.K2_GetActorRotation`)))
  (bind (_returnvalue_x _returnvalue_y _returnvalue_z) (`KismetMathLibrary.BreakVector` (`KismetMathLibrary.VLerp` (`KismetMathLibrary.MakeVector` _returnvalue_roll _returnvalue_pitch _returnvalue_yaw) (`KismetMathLibrary.MakeVector` (* (`self.RotationSpeed`) (`self.InputRoll`)) (* (`self.RotationSpeed`) (`self.InputPitch`)) (* (`self.RotationSpeed`) (`self.InputYaw`))) (* (`GameplayStatics.GetWorldDeltaSeconds`) 0.6))))
  (`self.K2_AddActorWorldRotation` (`KismetMathLibrary.MakeRotator` _returnvalue_x _returnvalue_y _returnvalue_z)))

(fn `UserConstructionScript`)