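; Player-controlled P-38 aircraft with throttle-driven movement and spinning propellers.
; BeginPlay adds the IMC_AceCombat Enhanced Input mapping when the controller is a BP_P38Controller, and IA_GroundControll adjusts a clamped CurrentSpeed.
; Tick spins both propellers at a constant rate and offsets the actor along world X by CurrentSpeed per frame, without delta-time scaling.
; The deceleration logic is unconnected.
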(event `self.ReceiveBeginPlay`
  (bind _asbp_p38controller (cast `/Game/Blueprints/P38/BP_P38Controller` (`GameplayStatics.GetPlayerController` 0)))
  (`EnhancedInputSubsystemInterface.AddMappingContext` (pcsubsystem `EnhancedInputLocalPlayerSubsystem` _asbp_p38controller) "/Game/Blueprints/Input/IMC_AceCombat.IMC_AceCombat" 0 (struct)))

(event `EnhancedInput|/Game/Blueprints/Input/IA_GroundControll`
  (params (ActionValue :type "Vector2D Structure") (ElapsedSeconds :type "Float (double-precision)") (TriggeredSeconds :type "Float (double-precision)") (InputAction :type "InputAction Object Reference" :default "/Game/Blueprints/Input/IA_GroundControll.IA_GroundControll"))
  (:`Triggered`
    (set `self.CurrentSpeed` (`KismetMathLibrary.FClamp` (+ (`self.CurrentSpeed`) (* ActionValue_X (* (`GameplayStatics.GetWorldDeltaSeconds`) (`self.Acceleration`)))) 0.0 (`self.MaxSpeed`)))))

(event `self.ReceiveTick`
  (params (DeltaSeconds :type "Float (single-precision)"))
  (`|ExecutionSequence`
    (:`then_0`
      ; Comment
      (`SceneComponent.K2_AddRelativeRotation` (`self.Right Propeller`) (`KismetMathLibrary.MakeRotator` (* (`GameplayStatics.GetWorldDeltaSeconds`) 5000.0)) false false)
      (`SceneComponent.K2_AddRelativeRotation` (`self.Left Propeller`) (`KismetMathLibrary.MakeRotator` (* (`GameplayStatics.GetWorldDeltaSeconds`) 5000.0)) false false))
    (:`then_2`
      (`self.K2_AddActorWorldOffset` (`KismetMathLibrary.MakeVector` (`self.CurrentSpeed`))))))

(fn `UserConstructionScript`)