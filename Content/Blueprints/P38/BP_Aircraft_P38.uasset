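; Player-flown P-38 aircraft with arcade-style flight, driven by Enhanced Input for roll, pitch, yaw and throttle.
; Each tick eases rotation rates toward input with FInterpTo, applies them as local rotations with yaw at half strength, and spins both propellers.
; Throttle changes speed with diminishing effect near the min and max limits, then the actor moves along its forward vector without sweep.
; A debug readout prints every tick.
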(event `self.ReceiveBeginPlay`
  ; Comment
  (bind _asbp_p38controller (cast `/Game/Blueprints/P38/BP_P38Controller` (`GameplayStatics.GetPlayerController` 0)))
  (`EnhancedInputSubsystemInterface.AddMappingContext` (pcsubsystem `EnhancedInputLocalPlayerSubsystem` _asbp_p38controller) "/Game/Blueprints/Input/IMC_AceCombat.IMC_AceCombat" 0 (struct)))

(event `EnhancedInput|/Game/Blueprints/Input/IA_YawAccel`
  (params (ActionValue :type "Vector2D Structure") (ElapsedSeconds :type "Float (double-precision)") (TriggeredSeconds :type "Float (double-precision)") (InputAction :type "InputAction Object Reference" :default "/Game/Blueprints/Input/IA_YawAccel.IA_YawAccel"))
  ; Comment
  (:`Triggered`
    (set `self.InputYaw` ActionValue_Y)
    (set `self.Accelerate` ActionValue_X))
  (:`Completed`
    (set `self.InputYaw` 0.0)
    (set `self.Accelerate` 0.0)))

(event `self.ReceiveTick`
  (params (DeltaSeconds :type "Float (single-precision)"))
  ; Event Tick
  (`|ExecutionSequence`
    (:`then_0`
      ;; Debug
      (`KismetSystemLibrary.PrintString` (`KismetTextLibrary.Conv_TextToString` (`|FormatText` "Roll : {Roll} \nPitch : {Pitch} \nYaw : {Yaw} \nSpeed : {Speed} \nAcceleration : {Acceleration }" (`self.InputRoll`) (`self.InputPitch`) (`self.InputYaw`) (`self.Current Speed`) (`self.Acceleration`))) true false (struct :`G` 0.66 :`B` 1.0 :`A` 1.0) 0.0))
    (:`then_1`
      ;; Comment
      (`self.UpdateRotation` (`self.Rotation Speed`) 2.0)
      (`self.RotatePropeller`))
    (:`then_2`
      ;; Forward Move
      (`self.UpdateSpeed`)
      (set `self.Current Speed` (`KismetMathLibrary.FClamp` (`self.Current Speed`) (`self.MinSpeed`) (`self.MaxSpeed`)))
      (`self.K2_AddActorWorldOffset` (* (`self.GetActorForwardVector`) (`self.Current Speed`) (`GameplayStatics.GetWorldDeltaSeconds`))))))

(event `EnhancedInput|/Game/Blueprints/Input/IA_RollPitch`
  (params (ActionValue :type "Vector2D Structure") (ElapsedSeconds :type "Float (double-precision)") (TriggeredSeconds :type "Float (double-precision)") (InputAction :type "InputAction Object Reference" :default "/Game/Blueprints/Input/IA_RollPitch.IA_RollPitch"))
  ; Comment
  (:`Triggered`
    (set `self.InputRoll` ActionValue_X)
    (set `self.InputPitch` ActionValue_Y))
  (:`Completed`
    (set `self.InputRoll` 0.0)
    (set `self.InputPitch` 0.0)))

(event `EnhancedInput|/Game/Blueprints/Input/IA_Fire`
  (params (ActionValue :type Boolean) (ElapsedSeconds :type "Float (double-precision)") (TriggeredSeconds :type "Float (double-precision)") (InputAction :type "InputAction Object Reference" :default "/Game/Blueprints/Input/IA_Fire.IA_Fire")))

(fn `RotatePropeller`
  (`SceneComponent.K2_AddRelativeRotation` (`self.Right Propeller`) (`KismetMathLibrary.MakeRotator` (* (`GameplayStatics.GetWorldDeltaSeconds`) -1800.0)) false false)
  (`SceneComponent.K2_AddRelativeRotation` (`self.Left Propeller`) (`KismetMathLibrary.MakeRotator` (* (`GameplayStatics.GetWorldDeltaSeconds`) -1800.0)) false false))

(fn `UpdateRotation`
  (params (RotationSpeed :type "Float (double-precision)") (InterpSpeed :type "Float (double-precision)"))
  (`|ExecutionSequence`
    (:`then_0`
      ; Roll
      (bind _output_get (set `self.CurrentRollRate` (`KismetMathLibrary.FInterpTo` (`self.CurrentRollRate`) (* (`self.InputRoll`) (`local.RotationSpeed`)) (`GameplayStatics.GetWorldDeltaSeconds`) (`local.InterpSpeed`))))
      (`self.K2_AddActorLocalRotation` (`KismetMathLibrary.MakeRotator` (* _output_get (`GameplayStatics.GetWorldDeltaSeconds`)))))
    (:`then_1`
      ; Pitch
      (bind _output_get_2 (set `self.CurrentPitchRate` (`KismetMathLibrary.FInterpTo` (`self.CurrentPitchRate`) (* (`self.InputPitch`) (`local.RotationSpeed`)) (`GameplayStatics.GetWorldDeltaSeconds`) (`local.InterpSpeed`))))
      (`self.K2_AddActorLocalRotation` (`KismetMathLibrary.MakeRotator` 0.0 (* _output_get_2 (`GameplayStatics.GetWorldDeltaSeconds`)))))
    (:`then_2`
      ; Yaw
      (bind _output_get_3 (set `self.CurrentYawRate` (`KismetMathLibrary.FInterpTo` (`self.CurrentYawRate`) (* (`self.InputYaw`) (`local.RotationSpeed`) 0.5) (`GameplayStatics.GetWorldDeltaSeconds`) (`local.InterpSpeed`))))
      (`self.K2_AddActorLocalRotation` (`KismetMathLibrary.MakeRotator` 0.0 0.0 (* _output_get_3 (`GameplayStatics.GetWorldDeltaSeconds`)))))))

(fn `UpdateSpeed`
  (if (> (`self.Accelerate`) 0.0)
    ; Acceleration
    (set `self.Acceleration` (* (`self.PropellingPower`) (/ (- (`self.MaxSpeed`) (`self.Current Speed`)) (`self.MaxSpeed`))))
    (set `self.Current Speed` (+ (`self.Current Speed`) (* (`self.Accelerate`) (`self.Acceleration`) (`GameplayStatics.GetWorldDeltaSeconds`))))
    (elif (< (`self.Accelerate`) 0.0)
      ; Deceleration
      (set `self.Acceleration` (* (`self.PropellingPower`) (/ (- (`self.Current Speed`) (`self.MinSpeed`)) (`self.MinSpeed`))))
      (set `self.Current Speed` (+ (`self.Current Speed`) (* (`self.Accelerate`) (`self.Acceleration`) (`GameplayStatics.GetWorldDeltaSeconds`)))))))

(fn `UserConstructionScript`)